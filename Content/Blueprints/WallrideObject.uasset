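; Wallride surface actor that launches the player along the wall and switches their movement state when a left or right rail collider overlaps it.
; The cross product Z sign of character mesh forward and a rotated wall vector picks forward or backward along the actor's axis.
; LaunchCharacter preserves horizontal speed, then the actor resets wallride time, grants an extra jump and registers itself to block repeat rides in the current combo.
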(event `self.ReceiveTick`
  (params (DeltaSeconds :type "Float (single-precision)")))

(event `self.WallSurface.OnComponentBeginOverlap`
  (params (OverlappedComponent :type "PrimitiveComponent Object Reference") (OtherActor :type "Actor Object Reference") (OtherComp :type "PrimitiveComponent Object Reference") (OtherBodyIndex :type Integer) (bFromSweep :type Boolean) (SweepResult :type "HitResult Structure (by ref)"))
  (bind _returnvalue (`self.GetActorForwardVector`))
  (bind _asthird_person_character (cast `/Game/ThirdPersonBP/Blueprints/ThirdPersonCharacter` (`GameplayStatics.GetPlayerPawn` 0) :!pure true))
  (bind _xy_speed (`/Game/ThirdPersonBP/Blueprints/ThirdPersonCharacter.Get XY Speed` _asthird_person_character))
  (bind (_returnvalue_x _returnvalue_y _returnvalue_z) (`KismetMathLibrary.BreakVector` (* _returnvalue (* _xy_speed -1.0))))
  (if (`KismetArrayLibrary.Array_Contains` (`/Game/ThirdPersonBP/Blueprints/ThirdPersonCharacter.Cannot Wallride In Current Combo` _asthird_person_character) self)
    _
    (elif (or (== OtherComp (`/Game/ThirdPersonBP/Blueprints/ThirdPersonCharacter.Rail Collider L` _asthird_person_character)) (== OtherComp (`/Game/ThirdPersonBP/Blueprints/ThirdPersonCharacter.Rail Collider R` _asthird_person_character)))
      (bind _left_ (`self.Determine whether to wallride left?` (`SceneComponent.K2_GetComponentLocation` OtherComp)))
      (if _left_
        (`Character.LaunchCharacter` _asthird_person_character (`KismetMathLibrary.MakeVector` _returnvalue_x _returnvalue_y _returnvalue_z) true true) ; Can't use std jump because !moving on grouind
        (else
          (`Character.LaunchCharacter` _asthird_person_character (`KismetMathLibrary.MakeVector` (.x (* _returnvalue _xy_speed)) (.y (* _returnvalue _xy_speed)) (.z (* _returnvalue _xy_speed))) true true) ; Can't use std jump because !moving on grouind
        ))
      (set `/Game/ThirdPersonBP/Blueprints/ThirdPersonCharacter.Movement State` "NewEnumerator2" _asthird_person_character)
      (set `/Game/ThirdPersonBP/Blueprints/ThirdPersonCharacter.Time On Wallride` 0.0 _asthird_person_character)
      (`KismetArrayLibrary.Array_Add` (`/Game/ThirdPersonBP/Blueprints/ThirdPersonCharacter.Cannot Wallride In Current Combo` _asthird_person_character) self)
      (set `/Game/ThirdPersonBP/Blueprints/ThirdPersonCharacter.Extra Jump From Wallriding?` true _asthird_person_character))))

(fn `Determine whether to wallride left?`
  (params (`Hit Location` :type "Vector Structure"))
  (returns (`Left?` :type Boolean))
  (locals (`Local Hit Location` :type "Vector Structure") (`Velocity Line Start World Space` :type "Vector Structure") (`Tangent Line End World Space` :type "Vector Structure") (`Tangent Line Start World Space` :type "Vector Structure") (`Tangent Line` :type "Vector Structure") (`Velocity Line End World Space` :type "Vector Structure") (`Velocity Line` :type "Vector Structure"))
  (bind _returnvalue (`KismetMathLibrary.Normal` (`KismetMathLibrary.GreaterGreater_VectorRotator` (`self.GetActorForwardVector`) (struct :`Yaw` -90.0))))
  (set `local.Local Hit Location` `Hit Location`)
  (set `local.Velocity Line Start World Space` (+ (* (`/Game/ThirdPersonBP/Blueprints/ThirdPersonCharacter.Get Mesh True Forward Vector` (cast `/Game/ThirdPersonBP/Blueprints/ThirdPersonCharacter` (`GameplayStatics.GetPlayerPawn` 0) :!pure true)) -100.0) (`local.Local Hit Location`)))
  (set `local.Tangent Line End World Space` (+ _returnvalue (`local.Local Hit Location`)))
  (set `local.Tangent Line Start World Space` (- (`local.Local Hit Location`) (* _returnvalue 100.0)))
  (set `local.Tangent Line` (- (`local.Tangent Line End World Space`) (`local.Tangent Line Start World Space`)))
  (set `local.Velocity Line End World Space` (`local.Local Hit Location`))
  (set `local.Velocity Line` (- (`local.Velocity Line End World Space`) (`local.Velocity Line Start World Space`)))
  (return (not (< (.z (`KismetMathLibrary.Cross_VectorVector` (`local.Velocity Line`) (`local.Tangent Line`))) 0.0))))

(fn `UserConstructionScript`
  (`self.Determine whether to wallride left?` (`self.K2_GetActorLocation`)))