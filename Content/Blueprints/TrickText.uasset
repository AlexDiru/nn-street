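; TrickText is a short-lived floating 3D text popup that displays a centered "Trick" label over the player.
; The construction script sets the text and a sub-second lifespan, so the actor removes itself.
; Each tick it re-anchors to the player pawn, rising along the pawn's up vector with its age, and rotates to face the ThirdPersonCharacter's FollowCamera.
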(event `self.ReceiveTick`
  (params (DeltaSeconds :type "Float (single-precision)"))
  (bind _returnvalue (`GameplayStatics.GetPlayerPawn` 0))
  (bind _returnvalue_location (`KismetMathLibrary.BreakTransform` (`self.GetTransform` _returnvalue)))
  (bind _returnvalue_2 (+ (* (`self.GetActorUpVector` _returnvalue) (* (`self.GetGameTimeSinceCreation`) 200.0)) _returnvalue_location))
  (`self.K2_SetActorLocationAndRotation` _returnvalue_2 (`KismetMathLibrary.FindLookAtRotation` _returnvalue_2 (`SceneComponent.K2_GetComponentLocation` (`/Game/ThirdPersonBP/Blueprints/ThirdPersonCharacter.FollowCamera` (cast `/Game/ThirdPersonBP/Blueprints/ThirdPersonCharacter` _returnvalue :!pure true)))) false true))

(fn `UserConstructionScript`
  (`TextRenderComponent.K2_SetText` (`self.TrickText`) (`|FormatText` "Trick"))
  (`TextRenderComponent.SetHorizontalAlignment` (`self.TrickText`) "EHTA_Center")
  (`self.SetLifeSpan` 0.6))